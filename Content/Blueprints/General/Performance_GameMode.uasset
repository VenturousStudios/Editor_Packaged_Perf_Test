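; Game mode that sets up a performance screen when play begins.
; It creates the Performance_Widget, flags it as a development build when its Scene reference is not valid, adds it to the viewport and shows the mouse cursor.
; After a short delay, it runs a console command that switches the game to a small windowed resolution.
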(event EventBeginPlay
  (Utilities|FlowControl|Sequence
    (:then_0
      (bind _returnvalue (UserInterface|CreateWidget "/Game/Blueprints/Performance_Widget.Performance_Widget_C" 0 (not (Utilities|IsValid (Variables|Default|GetScene)))))
      (UserInterface|Viewport|AddtoViewport _returnvalue 0)
      (Variables|/Script/Engine.PlayerController|SetbShowMouseCursor (Game|GetPlayerController 0) true))
    (:then_1
      (Utilities|FlowControl|Delay 0.5)
      (Development|ExecuteConsoleCommand "r.SetRes 960x540w" (Game|GetPlayerController 0)))))

(fn ConstructionScript)