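; Actor Blueprint named Actor_Spawn_Moderate, made up of placeholder custom events and stub functions, with no spawning logic.
; Three events call stub functions with literal or derived arguments, including one that truncates the X location from one function's output to feed another.
; The other events, the construction script and the function bodies are empty or return only default or zero values.
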(event Custom|CustomEvent_7
  (CallFunction|NewFunction3 "dagdgf" "testt"))

(event Custom|CustomEvent)

(event Custom|CustomEvent_5)

(event Custom|CustomEvent_6
  (bind _newparam2 (CallFunction|NewFunction2))
  (CallFunction|NewFunction4 (Math|Float|Truncate (.X (Math|Vector|BreakVector (.Location (Math|Transform|BreakTransform _newparam2)))))))

(event Custom|CustomEvent_1)

(event Custom|CustomEvent_2)

(event Custom|CustomEvent_3)

(event Custom|CustomEvent_4
  (CallFunction|NewFunction0 0.0 true))

(fn ConstructionScript)

(fn NewFunction)

(fn NewFunction0
  (params (NewParam :type Float%20%28double-precision%29) (NewParam1 :type Boolean)))

(fn NewFunction1
  (params (NewParam :type Transform) (NewParam1 :type Float%20%28double-precision%29) (NewParam2 :type Integer)))

(fn NewFunction2
  (return "" "" ""))

(fn NewFunction3
  (params (NewParam1 :type String) (NewParam2 :type Name))
  (return "0, 0, 0"))

(fn NewFunction4
  (params (NewParam :type Integer))
  (return "" "0, 0, 0"))